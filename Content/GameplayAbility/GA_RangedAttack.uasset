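; Gameplay ability for a ranged attack that fires a projectile at the avatar's combat target.
; On activation it turns the avatar toward the target through CombatInterface and plays the first attack montage, the only one currently supported.
; The montage's gameplay event triggers SpawnProjectile, using the montage's socket tag and the target's current location.
; It ends after a short post-spawn delay or when the montage completes, is interrupted or cancelled.
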(event Ability|EventActivateAbility
  (bind _returnvalue (Ability|GetAvatarActorfromActorInfo))
  (bind _returnvalue_2 (Class|EnemyInterface|GetCombatTarget(Message) _returnvalue))
  (bind _ascombat_interface (Utilities|Casting|CastToCombatInterface _returnvalue))
  (bind _output_get (Variables|Default|SetTargetLocation (Transformation|GetActorLocation _returnvalue_2)))
  (Class|CombatInterface|UpdateFacingTarget _ascombat_interface _output_get)
  (bind _returnvalue_3 (Class|CombatInterface|GetAttackMontages(Message) (Ability|GetAvatarActorfromActorInfo)))
  (Variables|Default|SetEventTag (.MontageTag (Utilities|Struct|BreakTaggedMontage (Utilities|Array|Get(acopy) _returnvalue_3))))
  (Variables|Default|SetSocket%20Tag (.SocketTag (Utilities|Struct|BreakTaggedMontage (Utilities|Array|Get(acopy) _returnvalue_3))))
  (|PlayMontageandWaitProxy "None" (.AttackMontage (Utilities|Struct|BreakTaggedMontage (Utilities|Array|Get(acopy) _returnvalue_3))) 1.0 "None" true 1.0 0.0
    (:then
      (Ability|Tasks|WaitGameplayEvent (Variables|Default|GetEventTag) 0 true
        (:EventReceived
          (Class|CombatInterface|GetCombatSocketLocation(Message) (Ability|GetAvatarActorfromActorInfo) (Variables|Default|GetEventTag))
          (bind _returnvalue_4 (Class|EnemyInterface|GetCombatTarget(Message) (Ability|GetAvatarActorfromActorInfo)))
          (Class|AuraProjectileSpell|SpawnProjectile (Transformation|GetActorLocation _returnvalue_4) (Variables|Default|GetSocket%20Tag))
          (Utilities|FlowControl|Delay 2.0)
          (Ability|EndAbility))))
    (:OnCompleted
      (Ability|EndAbility :!label _label))
    (:OnInterrupted
      (goto _label))
    (:OnCancelled
      (goto _label))))

(event Ability|EventOnEndAbility
  (params (bWasCancelled :type Boolean)))