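; BP_FlamePillar is an environment flame pillar whose fire light flickers continuously during play.
; On BeginPlay it randomly picks one of two flame intensity timelines and plays it from the start.
; Each timeline update sets the FireLight intensity to a base value times the curve's brightness.
; When a timeline finishes it picks again, giving an endless, varied flicker.
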(event Custom|StartTimeline1
  (bind _lightbrightness (Timeline|FlameIntensityTimeline_1 PlayFromStart)
    (:Update
      (Rendering|Components|Light|SetIntensity (Variables|Default|GetFireLight) (* (Variables|Default|GetBaseIntensityValue) _lightbrightness)))
    (:Finished
      (CallFunction|ChooseTimeline))))

(event Custom|StartTimeline2
  (bind _lightbrightness (Timeline|FlameIntensityTimeline_2 PlayFromStart)
    (:Update
      (Rendering|Components|Light|SetIntensity (Variables|Default|GetFireLight) (* (Variables|Default|GetBaseIntensityValue) _lightbrightness)))
    (:Finished
      (CallFunction|ChooseTimeline))))

(event Custom|chooseTimeline
  (switch int (Math|Random|RandomIntegerinRange 0 1)
    (:Default
      (CallFunction|StartTimeline2 :!label _label))
    (:0
      (CallFunction|StartTimeline1))
    (:1
      (goto _label))))

(event EventBeginPlay
  (CallFunction|ChooseTimeline))

(fn ConstructionScript)